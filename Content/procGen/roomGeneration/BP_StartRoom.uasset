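; BP_StartRoom is the starting room piece for procedural room generation, built on a parent Blueprint's construction logic.
; Its construction script runs the parent script, then flattens the Backward, Left, Right and Forward components along Z.
; The same loop also reduces the Floor component's Z scale, redundantly on every pass.
; The event graph holds only disabled placeholder events, so the Blueprint adds no runtime logic.
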(fn `UserConstructionScript`
  (`parent.UserConstructionScript`)
  (for _array_element (`|MakeArray` (`self.backward`) (`self.left`) (`self.right`) (`self.forward`))
    (`SceneComponent.SetRelativeScale3D` _array_element (1.0 1.0 0.1))
    (`SceneComponent.SetRelativeScale3D` (`self.floor`) (1.0 1.0 0.6))))