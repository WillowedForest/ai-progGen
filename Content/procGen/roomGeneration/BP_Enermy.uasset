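; BP_Enermy is a stationary-logic enemy actor that fires bullets in a cross pattern and destroys itself when touched by the player.
; A looping one-second timer started on BeginPlay calls shoot, which spawns BP_Bullet actors at its location, stepping world yaw by 90 degrees per shot.
; Overlap of Sphere1 with an actor tagged Player destroys the enemy.
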(event `self.ReceiveBeginPlay`
  (bind _returnvalue (`KismetSystemLibrary.K2_SetTimer` null "shoot" 1.0 true true))
  (set `self.shoot timer` _returnvalue))

(event `shoot`
  (for _ (range 4)
    (bind _output_get (set `self.Directions` (+ (`self.Directions`) 90.0)))
    (`|SpawnActorFromClass` "/Game/procGen/roomGeneration/BP_Bullet.BP_Bullet_C" (`KismetMathLibrary.MakeTransform` (`self.K2_GetActorLocation`) (`KismetMathLibrary.MakeRotator` 0.0 0.0 _output_get)) "Undefined" "MultiplyWithRoot" null null))
  (set `self.Directions` 0.0))

(event `self.Sphere1.OnComponentBeginOverlap`
  (params (OverlappedComponent :type "PrimitiveComponent Object Reference") (OtherActor :type "Actor Object Reference") (OtherComp :type "PrimitiveComponent Object Reference") (OtherBodyIndex :type Integer) (bFromSweep :type Boolean) (SweepResult :type "HitResult Structure (by ref)"))
  (if (`self.ActorHasTag` OtherActor "Player")
    (`self.K2_DestroyActor`)))

(fn `UserConstructionScript`)