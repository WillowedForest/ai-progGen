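; Dungeon generator actor that builds a connected grid layout of room actors on BeginPlay.
; It pads the RoomsToSpawn quota map with empty rooms up to RoomAmount, then random-walks in four directions from a start room.
; Free cells get randomly picked room classes, occupied cells are linked and walked through, and the final spawn is BP_LastRoom.
; Rooms record their connections, and each runs CreatePath once generation finishes.
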(event `self.ReceiveBeginPlay`
  (bind _roomstospawn (`self.RoomsToSpawn`))
  (bind _keys (`BlueprintMapLibrary.Map_Keys` _roomstospawn))
  (for _array_element _keys
    (set `self.tempCount` (+ (`self.tempCount`) (`BlueprintMapLibrary.Map_Find` _roomstospawn _array_element))))
  (bind _output_get (set `self.nonEmptyRoomCount` (`self.tempCount`)))
  (`BlueprintMapLibrary.Map_Add` (`self.RoomsToSpawn`) "/Game/procGen/roomGeneration/BP_EmptyRoom.BP_EmptyRoom_C" (- (`self.RoomAmount`) _output_get))
  (bind _asbp_game_instance (cast `/Game/blueprints/BP_GameInstance` (`GameplayStatics.GetGameInstance`)))
  (set `self.Game Instance` _asbp_game_instance)
  (set `self.RoomsLeft` (`self.RoomAmount`))
  (bind _returnvalue (`|SpawnActorFromClass` "/Game/procGen/roomGeneration/BP_StartRoom.BP_StartRoom_C" (`KismetMathLibrary.MakeTransform` (0.0 0.0 0.0)) "Undefined" "MultiplyWithRoot" null (`self.Game Instance`) null))
  (bind _output_get_2 (set `self.StartRoom` _returnvalue))
  (bind (_returnvalue_x _returnvalue_y) (`KismetMathLibrary.BreakVector` (`self.K2_GetActorLocation` _returnvalue)))
  (`BlueprintMapLibrary.Map_Add` (`self.Rooms`) _output_get_2 (`KismetMathLibrary.MakeVector2D` _returnvalue_x _returnvalue_y))
  (set `self.LastRoom` (`self.StartRoom`))
  (bind _result (`/Engine/EditorBlueprintResources/StandardMacros.DecrementInt` (`self.RoomsLeft`))
    (:`  `
      (set `self.RoomsLeft` _result)
      (if (> (`self.RoomsLeft`) 0) :!label _label
        (`self.SpawnRandomRooms`)
        (goto _label)
        (else
          (bind _keys_2 (`BlueprintMapLibrary.Map_Keys` (`self.Rooms`)))
          (for _array_element_2 _keys_2
            (`/Game/procGen/roomGeneration/BP_RoomParent.CreatePath` _array_element_2)))))))

(fn `SpawnRandomRooms`
  (locals (PotentialLocation :type "Vector2D Structure") (CurrentRoom :type "/Game/procGen/roomGeneration/BP_RoomParent Object Reference"))
  (bind (_gridsize_x _gridsize_y) (`KismetMathLibrary.BreakVector2D` (`self.GridSize`)))
  (bind (_potentiallocation_x _potentiallocation_y) (`KismetMathLibrary.BreakVector2D` (`local.PotentialLocation`)))
  (bind _rooms (`self.Rooms`))
  (bind _roomstospawn (`self.RoomsToSpawn`))
  (bind _gridsize_x_2 (`KismetMathLibrary.BreakVector2D` (`self.GridSize`)))
  (bind _gridsize_x_3 (`KismetMathLibrary.BreakVector2D` (`self.GridSize`)))
  (bind (_gridsize_x_4 _gridsize_y_2) (`KismetMathLibrary.BreakVector2D` (`self.GridSize`)))
  (bind (_potentiallocation_x_2 _potentiallocation_y_2) (`KismetMathLibrary.BreakVector2D` (`local.PotentialLocation`)))
  (bind _value (`BlueprintMapLibrary.Map_Find` (`self.Rooms`) (`self.LastRoom`)))
  (bind (_x _y) (`KismetMathLibrary.BreakVector2D` _value))
  (bind (_x_2 _y_2) (`KismetMathLibrary.BreakVector2D` _value))
  (bind (_x_3 _y_3) (`KismetMathLibrary.BreakVector2D` _value))
  (bind (_x_4 _y_4) (`KismetMathLibrary.BreakVector2D` _value))
  (bind (_key _value_2) (`BlueprintMapLibrary.Map_GetKeyValueByIndex` _roomstospawn (`KismetMathLibrary.RandomInteger` (`BlueprintMapLibrary.Map_Length` _roomstospawn))))
  (bind _output_get (set `local.PotentialLocation` (select `int` (`KismetMathLibrary.RandomIntegerInRange` 0 3) :`0` (`KismetMathLibrary.MakeVector2D` (+ _x_3 _gridsize_x_3) _y_3) :`1` (`KismetMathLibrary.MakeVector2D` _x_4 (+ _y_4 _gridsize_y_2)) :`2` (`KismetMathLibrary.MakeVector2D` (- _x_2 _gridsize_x_2) _y_2) :`3` (`KismetMathLibrary.MakeVector2D` _x (- _y _gridsize_y)))))
  (bind _values (`BlueprintMapLibrary.Map_Values` (`self.Rooms`)))
  (if (`KismetArrayLibrary.Array_Contains` _values _output_get)
    (bind _values_2 (`BlueprintMapLibrary.Map_Values` _rooms))
    (bind _keys (`BlueprintMapLibrary.Map_Keys` _rooms))
    (bind _output_get_2 (set `local.CurrentRoom` (`|GetArrayItem` _keys (`KismetArrayLibrary.Array_Find` _values_2 (`local.PotentialLocation`)))))
    (`BlueprintSetLibrary.Set_Add` (`/Game/procGen/roomGeneration/BP_RoomParent.RoomConections` _output_get_2) (`self.LastRoom`))
    (`BlueprintSetLibrary.Set_Add` (`/Game/procGen/roomGeneration/BP_RoomParent.RoomConections` (`self.LastRoom`)) (`local.CurrentRoom`))
    (set `self.LastRoom` (`local.CurrentRoom`))
    (elif (== (`self.RoomsLeft`) 1)
      (bind _returnvalue (`|SpawnActorFromClass` "/Game/procGen/roomGeneration/BP_LastRoom.BP_LastRoom_C" (`KismetMathLibrary.MakeTransform` (`KismetMathLibrary.MakeVector` _potentiallocation_x_2 _potentiallocation_y_2)) "Undefined" "MultiplyWithRoot" null (`self.Game Instance`) null))
      (bind _output_get_3 (set `local.CurrentRoom` _returnvalue))
      (bind (_returnvalue_x _returnvalue_y) (`KismetMathLibrary.BreakVector` (`self.K2_GetActorLocation` _returnvalue)))
      (`BlueprintMapLibrary.Map_Add` (`self.Rooms`) _output_get_3 (`KismetMathLibrary.MakeVector2D` _returnvalue_x _returnvalue_y))
      (bind _result (`/Engine/EditorBlueprintResources/StandardMacros.DecrementInt` (`self.RoomsLeft`))
        (:`  `
          (set `self.RoomsLeft` _result)
          (`BlueprintSetLibrary.Set_Add` (`/Game/procGen/roomGeneration/BP_RoomParent.RoomConections` (`local.CurrentRoom`)))
          (`BlueprintSetLibrary.Set_Add` (`/Game/procGen/roomGeneration/BP_RoomParent.RoomConections` (`self.LastRoom`)) (`local.CurrentRoom`))
          (set `self.LastRoom` (`local.CurrentRoom`))))
      (elif (not (<= _value_2 0))
        (`/Engine/EditorBlueprintResources/StandardMacros.DecrementInt` _value_2
          (:`  `
            (bind _returnvalue_2 (`|SpawnActorFromClass` _key (`KismetMathLibrary.MakeTransform` (`KismetMathLibrary.MakeVector` _potentiallocation_x _potentiallocation_y)) "Undefined" "MultiplyWithRoot" null (`self.Game Instance`) null))
            (bind _output_get_4 (set `local.CurrentRoom` _returnvalue_2))
            (bind (_returnvalue_x_2 _returnvalue_y_2) (`KismetMathLibrary.BreakVector` (`self.K2_GetActorLocation` _returnvalue_2)))
            (`BlueprintMapLibrary.Map_Add` (`self.Rooms`) _output_get_4 (`KismetMathLibrary.MakeVector2D` _returnvalue_x_2 _returnvalue_y_2))
            (bind _result_2 (`/Engine/EditorBlueprintResources/StandardMacros.DecrementInt` (`self.RoomsLeft`))
              (:`  `
                (set `self.RoomsLeft` _result_2)
                (`BlueprintSetLibrary.Set_Add` (`/Game/procGen/roomGeneration/BP_RoomParent.RoomConections` (`local.CurrentRoom`)) (`self.LastRoom`))
                (`BlueprintSetLibrary.Set_Add` (`/Game/procGen/roomGeneration/BP_RoomParent.RoomConections` (`self.LastRoom`)) (`local.CurrentRoom`))
                (set `self.LastRoom` (`local.CurrentRoom`))))))))))

(fn `UserConstructionScript`)