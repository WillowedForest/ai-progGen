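; BP_RoomParent is a base room Blueprint for procedural generation that opens paths toward its connected rooms.
; On BeginPlay it stores its world X and Y location as Coordinates.
; CreatePath compares these with each room in RoomConections and destroys the Forward, Backward, Left or Right component facing that neighbor.
; An X difference takes priority over Y, with +X mapped to Forward and +Y to Left.
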(event `self.ReceiveBeginPlay`
  (bind (_returnvalue_x _returnvalue_y) (`KismetMathLibrary.BreakVector` (`self.K2_GetActorLocation`)))
  (set `self.Coordinates` (`KismetMathLibrary.MakeVector2D` _returnvalue_x _returnvalue_y)))

(event `CreatePath`
  (bind _coordinates_x (`KismetMathLibrary.BreakVector2D` (`self.Coordinates`)))
  (bind _coordinates_x_2 (`KismetMathLibrary.BreakVector2D` (`self.Coordinates`)))
  (bind (_coordinates_x_3 _coordinates_y) (`KismetMathLibrary.BreakVector2D` (`self.Coordinates`)))
  (bind _result (`BlueprintSetLibrary.Set_ToArray` (`self.RoomConections`)))
  (for _array_element _result
    (bind _coordinates_x_4 (`KismetMathLibrary.BreakVector2D` (`/Game/procGen/roomGeneration/BP_RoomParent.Coordinates` _array_element)))
    (if (!= _coordinates_x_4 _coordinates_x_2)
      (bind _coordinates_x_5 (`KismetMathLibrary.BreakVector2D` (`/Game/procGen/roomGeneration/BP_RoomParent.Coordinates` _array_element)))
      (if (> _coordinates_x_5 _coordinates_x)
        (`ActorComponent.K2_DestroyComponent` (`self.forward`))
        (else
          (`ActorComponent.K2_DestroyComponent` (`self.backward`))))
      (else
        (bind (_coordinates_x_6 _coordinates_y_2) (`KismetMathLibrary.BreakVector2D` (`/Game/procGen/roomGeneration/BP_RoomParent.Coordinates` _array_element)))
        (if (> _coordinates_y_2 _coordinates_y)
          (`ActorComponent.K2_DestroyComponent` (`self.left`))
          (else
            (`ActorComponent.K2_DestroyComponent` (`self.right`))))))))

(fn `UserConstructionScript`)