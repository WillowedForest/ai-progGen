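; BP_Chest is a chest that rolls random loot each time a Player-tagged character overlaps its box.
; Each overlap clears DroppedLoot, picks one random DT_LootTabe row and applies its weighted drop chance and a random quantity.
; Any result is added to the running totals in the character's Loot map and printed as a pickup message.
; The chest has no opened state, so re-entering rolls again.
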(event `self.Box.OnComponentBeginOverlap`
  (params (OverlappedComponent :type "PrimitiveComponent Object Reference") (OtherActor :type "Actor Object Reference") (OtherComp :type "PrimitiveComponent Object Reference") (OtherBodyIndex :type Integer) (bFromSweep :type Boolean) (SweepResult :type "HitResult Structure (by ref)"))
  (bind _droppedloot (`self.DroppedLoot`))
  (bind _loot (`/Game/ThirdPerson/Blueprints/BP_ThirdPersonCharacter.Loot` (`self.As BP Third Person Character`)))
  (if (`self.ActorHasTag` OtherActor "Player")
    (bind _asbp_third_person_character (cast `/Game/ThirdPerson/Blueprints/BP_ThirdPersonCharacter` OtherActor))
    (set `self.As BP Third Person Character` _asbp_third_person_character)
    (`BlueprintMapLibrary.Map_Clear` (`self.DroppedLoot`))
    (`self.GenerateRandomLoot`)
    (bind _keys (`BlueprintMapLibrary.Map_Keys` _droppedloot))
    (for _array_element _keys
      (bind _value (`BlueprintMapLibrary.Map_Find` _droppedloot _array_element))
      (`BlueprintMapLibrary.Map_Add` _loot _array_element (+ (`BlueprintMapLibrary.Map_Find` _loot _array_element) _value))
      (`KismetSystemLibrary.PrintString` (`KismetStringLibrary.Concat_StrStr` "picked up" (`KismetStringLibrary.Conv_IntToString` _value) "" (`KismetStringLibrary.Conv_NameToString` _array_element))))))

(event `GenerateRandomLoot`
  (bind _outrownames (`DataTableFunctionLibrary.GetDataTableRowNames` "/Game/procGen/chest/DT_LootTabe.DT_LootTabe"))
  (bind _returnvalue (`|GetDataTableRow` "/Game/procGen/chest/DT_LootTabe.DT_LootTabe" (`|GetArrayItem` _outrownames (`KismetMathLibrary.RandomInteger` (`KismetArrayLibrary.Array_Length` _outrownames))))
    (:`then`
      (bind (_lootid _quontity _dropchance) (break `/Game/procGen/chest/BPS_LootDrops` _returnvalue))
      (if (`KismetMathLibrary.RandomBoolWithWeight` (/ _dropchance 10.0))
        (bind _returnvalue_2 (`KismetMathLibrary.RandomInteger` _quontity))
        (if (!= _returnvalue_2 0)
          (`BlueprintMapLibrary.Map_Add` (`self.DroppedLoot`) _lootid _returnvalue_2))))))

(fn `UserConstructionScript`)